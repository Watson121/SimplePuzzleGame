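; BP_Paper_Pickup is a collectible paper item that the player picks up by walking into it.
; The actor slowly spins around its vertical axis on Tick.
; When its Box overlaps a BP_TopDownCharacter, it sends a Use message, and the Use event increments that player's bits of paper and destroys the pickup.
; CanBeUsed always returns false.
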(event `self.ReceiveTick`
  (params (DeltaSeconds :type "Float (single-precision)"))
  (`self.K2_AddActorWorldRotation` (* (struct :`Yaw` 1.0) (* DeltaSeconds 10.0))))

(event `self.Box.OnComponentBeginOverlap`
  (params (OverlappedComponent :type "PrimitiveComponent Object Reference") (OtherActor :type "Actor Object Reference") (OtherComp :type "PrimitiveComponent Object Reference") (OtherBodyIndex :type Integer) (bFromSweep :type Boolean) (SweepResult :type "HitResult Structure (by ref)"))
  (bind _asbp_top_down_character (cast `/Game/TopDown/Blueprints/BP_TopDownCharacter` OtherActor))
  (message `InteractionInterface.Use` self _asbp_top_down_character))

(event `InteractionInterface.Use`
  (params (player :type "SimplePuzzleGameCharacter Object Reference"))
  (`SimplePuzzleGameCharacter.IncreaseBitsOfPaper` player)
  (`self.K2_DestroyActor`))

(fn `CanBeUsed`
  (returns (ReturnValue :type Boolean))
  (return false))

(fn `UserConstructionScript`)